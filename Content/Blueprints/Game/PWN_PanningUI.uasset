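; Pawn for a panning thumbnail UI, controlled by Leap Motion or keyboard, that opens a slide viewer when a BP_PannedWidget is clicked.
; While slides are closed, a non-open hand drives the mouse cursor through Leap-to-screen mapping.
; While open, open-hand swipes or arrow keys page and close the slides.
; Opening hides the cursor and starts a Tick lerp of the background material's emissive strength, targeted by open state.
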(event `self.ReceiveBeginPlay`
  (bind _asbp_game_instance (cast `/Game/Blueprints/Game/BP_GameInstance` (`GameplayStatics.GetGameInstance`)))
  (set `self.GameInstanceRef` _asbp_game_instance)
  (`LeapController.EnableGesture` (`self.LeapController`) "GESTURE_TYPE_SWIPE" true)
  (bind _returnvalue (`|CreateWidget` "/Game/Blueprints/UI/PanningWidget/W_OpenSlideContainer.W_OpenSlideContainer_C" (`GameplayStatics.GetPlayerController` 0)))
  (`UserWidget.AddToViewport` _returnvalue 0)
  (set `self.MainUISlide` (`/Game/Blueprints/UI/PanningWidget/W_OpenSlideContainer.OpenSlide` _returnvalue))
  (bind _outactors (`GameplayStatics.GetAllActorsOfClass` "/Game/Blueprints/Panning/BP_PannedWidget.BP_PannedWidget_C"))
  (bind _output_get (set `self.ThumbnailActors` _outactors))
  (for _array_element _output_get
    (add `/Game/Blueprints/Panning/BP_PannedWidget.OnWidgetClicked` _array_element (delegate `OpenMainUI`))
    (set `/Game/Blueprints/Panning/BP_PannedWidget.IsHoverEnabled` (`.UseLeapMotion_1_9C9D09F642CD68D7D30520AA880A19A8` (break `/Game/Blueprints/Game/S_GameSettings` (`/Game/Blueprints/Game/BP_GameInstance.CurrentGameSettings` (`self.GameInstanceRef`)))) _array_element)))

(event `OpenMainUI`
  (params (WidgetIdx :type Integer))
  (`/Game/Blueprints/UI/PanningWidget/W_OpenSlide.OpenSlide` (`self.MainUISlide`) WidgetIdx)
  (set `PlayerController.bShowMouseCursor` false (`GameplayStatics.GetPlayerController` 0))
  (set `self.IsAnimatingBG` true))

(event `LeapEventInterface.LeapHandMoved`
  (params (hand :type "LeapHand Object Reference"))
  (if (`self.IsInputEnabled`)
    (if (not (== hand (`self.TrackedHand`)))
      (set `self.TrackedHand` hand))
    (bind (_fingers _open) (`self.IsHandOpen` (`self.TrackedHand`)))
    (if (not (or (`/Game/Blueprints/UI/PanningWidget/W_OpenSlide.IsOpen` (`self.MainUISlide`)) _open))
      (bind _returnvalue (`LeapFingerList.GetPointableById` _fingers 0))
      (bind _returnvalue_2 (`LeapPointable.Frame` _returnvalue))
      (bind _returnvalue_3 (`LeapFrame.InteractionBox` _returnvalue_2))
      (bind (_x _y) (`self.LeapToScreen` _returnvalue_3 (`LeapPointable.StabilizedTipPosition` _returnvalue)))
      (`PlayerController.SetMouseLocation` (`GameplayStatics.GetPlayerController` 0) _x _y))))

(event `Key|Left`
  (params (Key :type "Key Structure" :default "LeapLeftPinch"))
  (:`Pressed`
    (`/Game/Blueprints/UI/PanningWidget/W_OpenSlide.ShowNextSlide` (`self.MainUISlide`) :!label _label)))

(event `LeapEventInterface.SwipeGestureDetected`
  (params (gesture :type "LeapSwipeGesture Object Reference"))
  (bind _returnvalue (`LeapGesture.Hands` gesture))
  (bind _returnvalue_2 (`LeapHandList.Frontmost` _returnvalue))
  (bind (_fingers _open) (`self.IsHandOpen` _returnvalue_2))
  (if (and _open (`/Game/Blueprints/UI/PanningWidget/W_OpenSlide.IsOpen` (`self.MainUISlide`)))
    (switch `LeapBasicDirection` (`LeapSwipeGesture.BasicDirection` gesture)
      (:`DIRECTION_LEFT`
        (goto _label))
      (:`DIRECTION_RIGHT`
        (`/Game/Blueprints/UI/PanningWidget/W_OpenSlide.ShowPrevSlide` (`self.MainUISlide`) :!label _label_2))
      (:`DIRECTION_DOWN`
        (`self.CloseMainUI`)))))

(event `Key|Up`
  (params (Key :type "Key Structure" :default "LeapLeftPinch"))
  (:`Pressed`
    (`/Game/Blueprints/UI/PanningWidget/W_OpenSlide.Close` (`self.MainUISlide`) :!label _label_3)
    (set `self.CloseCounter` 0)
    (set `PlayerController.bShowMouseCursor` true (`GameplayStatics.GetPlayerController` 0))))

(event `Key|Right`
  (params (Key :type "Key Structure" :default "LeapLeftPinch"))
  (:`Pressed`
    (goto _label_2)))

(event `CloseMainUI`
  (goto _label_3))

(event `InitBG`
  (bind _returnvalue (`KismetMaterialLibrary.CreateDynamicMaterialInstance` "/Game/Materials/Animated/Info/MI_PanningScreen.MI_PanningScreen"))
  (bind _output_get (set `self.BG_Mat` _returnvalue))
  (`PrimitiveComponent.SetMaterial` (`StaticMeshActor.StaticMeshComponent` (`self.Background`)) 0 _output_get))

(event `self.ReceiveTick`
  (params (DeltaSeconds :type "Float (single-precision)"))
  (bind _bg_mat (`self.BG_Mat`))
  (bind _currentbgemissive (`self.CurrentBGEmissive`))
  (bind _returnvalue (* DeltaSeconds (`self.BGLerpSpeed`)))
  (if (`self.IsAnimatingBG`)
    (if (`/Game/Blueprints/UI/PanningWidget/W_OpenSlide.IsOpen` (`self.MainUISlide`))
      (bind _output_get (set `self.CurrentBGEmissive` (`KismetMathLibrary.Lerp` _currentbgemissive 0.6 _returnvalue)))
      (`MaterialInstanceDynamic.SetScalarParameterValue` _bg_mat "Emissive Strength" _output_get)
      (if (`KismetMathLibrary.NearlyEqual_FloatFloat` _output_get 0.6 0.001)
        (set `self.IsAnimatingBG` false))
      (else
        (bind _output_get_2 (set `self.CurrentBGEmissive` (`KismetMathLibrary.Lerp` _currentbgemissive 3.5 _returnvalue)))
        (`MaterialInstanceDynamic.SetScalarParameterValue` _bg_mat "Emissive Strength" _output_get_2)
        (if (`KismetMathLibrary.NearlyEqual_FloatFloat` _output_get_2 3.5 0.001)
          (set `self.IsAnimatingBG` false))))))

(fn `UserConstructionScript`)