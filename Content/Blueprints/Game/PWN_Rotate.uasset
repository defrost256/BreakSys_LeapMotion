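; Player pawn for inspecting BP_BreakSystem actors, rotating a grabbed one by mouse or Leap Motion hand.
; GrabActor disables clicking on all breaks, swaps their labels for a screen-space text widget and dims the background material's emissive through Tick; ExitActor reverses this.
; An open Leap hand rotates by palm movement or exits when turned sideways, while fewer extended fingers drive the mouse cursor.
; Right-mouse drag also rotates, and left click exits.
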(event `self.ReceiveBeginPlay`
  (bind _outactors (`GameplayStatics.GetAllActorsOfClass` "/Game/Blueprints/Breaks/BP_BreakSystem.BP_BreakSystem_C"))
  (bind _output_get (set `self.Breaks` _outactors))
  (for _array_element _output_get
    (set `/Game/Blueprints/Breaks/BP_BreakSystem.ControllingPawn` self _array_element)
    (bind _returnvalue (`|CreateWidget` "/Game/Blueprints/UI/W_ScreenSpaceBreakText.W_ScreenSpaceBreakText_C" (`GameplayStatics.GetPlayerController` 0)))
    (bind _output_get_2 (set `self.BreakTextMain` _returnvalue))
    (`UserWidget.AddToViewport` _output_get_2 0)))

(event `Key|RightMouseButton`
  (params (Key :type "Key Structure" :default "LeapLeftPinch"))
  (bind _hasgrabbedactor (`self.HasGrabbedActor`))
  (:`Pressed`
    (if _hasgrabbedactor
      (set `self.IsMouseGrabbed` true)))
  (:`Released`
    (if _hasgrabbedactor
      (set `self.IsMouseGrabbed` false))))

(event `InputAxisKey|MouseX`
  (params (AxisValue :type "Float (single-precision)"))
  (if (and (`self.IsMouseGrabbed`) (`self.HasGrabbedActor`))
    (`/Game/Blueprints/Breaks/BP_BreakSystem.AddToTargetRotation` (`self.CurrentlyGrabbedActor`) (`KismetMathLibrary.MakeRotator` 0.0 0.0 (* AxisValue (`self.MouseRotationSpeed`) -1.0)))))

(event `InputAxisKey|MouseY`
  (params (AxisValue :type "Float (single-precision)"))
  (if (and (`self.IsMouseGrabbed`) (`self.HasGrabbedActor`))
    (`/Game/Blueprints/Breaks/BP_BreakSystem.AddToTargetRotation` (`self.CurrentlyGrabbedActor`) (`KismetMathLibrary.MakeRotator` 0.0 (* (`self.MouseRotationSpeed`) AxisValue -1.0)))))

(event `Key|LeftMouseButton` :consume false
  (params (Key :type "Key Structure" :default "LeapLeftPinch"))
  (:`Pressed`
    (if (`self.HasGrabbedActor`)
      (`self.ExitActor`))))

(event `GrabActor`
  (params (Actor :type "/Game/Blueprints/Breaks/BP_BreakSystem Object Reference"))
  (set `self.CurrentlyGrabbedActor` Actor)
  (set `self.HasGrabbedActor` true)
  (for _array_element (`self.Breaks`)
    (set `/Game/Blueprints/Breaks/BP_BreakSystem.CanBeClicked` false _array_element)
    (bind _asbreak_text (cast `/Game/Blueprints/UI/BreakText` (`WidgetComponent.GetUserWidgetObject` (`/Game/Blueprints/Breaks/BP_BreakSystem.Text` _array_element))))
    (`/Game/Blueprints/UI/BreakText.Close` _asbreak_text))
  (`/Game/Blueprints/UI/W_ScreenSpaceBreakText.SetText` (`self.BreakTextMain`) (`/Game/Blueprints/Breaks/BP_BreakSystem.HeaderText` (`self.CurrentlyGrabbedActor`)) (`/Game/Blueprints/Breaks/BP_BreakSystem.BodyText` (`self.CurrentlyGrabbedActor`)))
  (`/Game/Blueprints/UI/W_ScreenSpaceBreakText.Open` (`self.BreakTextMain`))
  (set `self.IsAnimatingBG` true))

(event `LeapEventInterface.LeapHandMoved`
  (params (hand :type "LeapHand Object Reference"))
  (bind _trackedhand (`self.TrackedHand`))
  ;[1 1 1] Handle Leap motion input
  (if (`self.IsInputEnabled`)
    (if (not (== hand (`self.TrackedHand`)))
      (set `self.TrackedHand` hand))
    (bind _returnvalue (`LeapHand.Fingers` (`self.TrackedHand`)))
    (bind _returnvalue_2 (`LeapFingerList.Extended` _returnvalue))
    (if (> (`LeapFingerList.Count` _returnvalue_2) 2)
      (if (and (`self.IsPalmPosSet`) (`self.HasGrabbedActor`))
        (if (> (.x (`LeapHand.PalmNormal` _trackedhand)) 0.8)
          (`self.ExitActor`)
          (else
            (`self.RotateWithHand` _trackedhand)))
        (else
          (set `self.PrevPalmPosition` (`LeapHand.StabilizedPalmPosition` _trackedhand))
          (set `self.IsPalmPosSet` true)))
      (else
        (set `self.IsPalmPosSet` false)
        (bind _returnvalue_3 (`LeapFingerList.GetPointableById` _returnvalue_2 0))
        (`self.PointWithFinger` _returnvalue_3)))))

(event `InitBG`
  (bind _returnvalue (`KismetMaterialLibrary.CreateDynamicMaterialInstance` "/Game/Materials/Animated/Background/MI_Background.MI_Background"))
  (bind _output_get (set `self.BG_Mat` _returnvalue))
  (`PrimitiveComponent.SetMaterial` (`StaticMeshActor.StaticMeshComponent` (`self.Background`)) 0 _output_get))

(event `self.ReceiveTick`
  (params (DeltaSeconds :type "Float (single-precision)"))
  (bind _bg_mat (`self.BG_Mat`))
  (bind _currentbgemissive (`self.CurrentBGEmissive`))
  (bind _returnvalue (* DeltaSeconds (`self.BGLerpSpeed`)))
  (if (`self.IsAnimatingBG`)
    (if (`self.HasGrabbedActor`)
      (bind _output_get (set `self.CurrentBGEmissive` (`KismetMathLibrary.Lerp` _currentbgemissive 0.5 _returnvalue)))
      (`MaterialInstanceDynamic.SetScalarParameterValue` _bg_mat "Emissive Strength" _output_get)
      (if (`KismetMathLibrary.NearlyEqual_FloatFloat` _output_get 0.5 0.001)
        (set `self.IsAnimatingBG` false))
      (else
        (bind _output_get_2 (set `self.CurrentBGEmissive` (`KismetMathLibrary.Lerp` _currentbgemissive 12.0 _returnvalue)))
        (`MaterialInstanceDynamic.SetScalarParameterValue` _bg_mat "Emissive Strength" _output_get_2)
        (if (`KismetMathLibrary.NearlyEqual_FloatFloat` _output_get_2 12.0 0.001)
          (set `self.IsAnimatingBG` false))))))

(fn `ExitActor`
  (if (`self.HasGrabbedActor`)
    (bind _success (`/Game/Blueprints/Breaks/BP_BreakSystem.ReturnToPosition` (`self.CurrentlyGrabbedActor`)))
    (if _success
      (set `self.HasGrabbedActor` false)
      (for _array_element (`self.Breaks`)
        (set `/Game/Blueprints/Breaks/BP_BreakSystem.CanBeClicked` true _array_element)
        (bind _asbreak_text (cast `/Game/Blueprints/UI/BreakText` (`WidgetComponent.GetUserWidgetObject` (`/Game/Blueprints/Breaks/BP_BreakSystem.Text` _array_element))))
        (`/Game/Blueprints/UI/BreakText.Open` _asbreak_text))
      (`/Game/Blueprints/UI/W_ScreenSpaceBreakText.Close` (`self.BreakTextMain`))
      (set `self.IsAnimatingBG` true))))

(fn `PointWithFinger`
  (params (Finger :type "LeapPointable Object Reference"))
  (bind _returnvalue (`LeapPointable.Frame` Finger))
  (bind _returnvalue_2 (`LeapFrame.InteractionBox` _returnvalue))
  (bind (_x _y) (`self.ConvertLeapToScreen` _returnvalue_2 (`LeapPointable.StabilizedTipPosition` Finger)))
  (`PlayerController.SetMouseLocation` (`GameplayStatics.GetPlayerController` 0) _x _y))

(fn `RotateWithHand`
  (params (Hand :type "LeapHand Object Reference"))
  (bind _stabilizedpalmposition (`LeapHand.StabilizedPalmPosition` Hand))
  (if (and (`self.IsRotateEnabled`) (`self.HasGrabbedActor`))
    (`/Game/Blueprints/Breaks/BP_BreakSystem.AddToTargetRotation` (`self.CurrentlyGrabbedActor`) (`KismetMathLibrary.MakeRotator` (.x (* (- _stabilizedpalmposition (`self.PrevPalmPosition`)) (`self.LeapRotationSpeed`))) (.z (* (- _stabilizedpalmposition (`self.PrevPalmPosition`)) (`self.LeapRotationSpeed`))) (.y (* (- _stabilizedpalmposition (`self.PrevPalmPosition`)) (`self.LeapRotationSpeed`)))))
    (set `self.PrevPalmPosition` _stabilizedpalmposition)))

(fn `UserConstructionScript`)