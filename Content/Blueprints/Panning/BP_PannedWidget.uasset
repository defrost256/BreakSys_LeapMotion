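; BP_PannedWidget is an actor showing a W_PanningThumbnail widget that scrolls along world X at a set speed as a clickable slide.
; Successive sphere overlaps open the thumbnail, close it, then shift the actor by a respawn distance, allowing it to be recycled in a loop.
; A left click, or an optional timed hover that accumulates on Tick, calls OnWidgetClicked with the slide index.
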(event `self.ReceiveBeginPlay`
  (bind _asw_panning_thumbnail (cast `/Game/Blueprints/UI/PanningWidget/W_PanningThumbnail` (`WidgetComponent.GetUserWidgetObject` (`self.Widget`))))
  (bind _output_get (set `self.ThumbnailWidget` _asw_panning_thumbnail))
  (`/Game/Blueprints/UI/PanningWidget/W_PanningThumbnail.SetThumbnail` _output_get (`self.ThumbnailTexture`)))

(event `self.ReceiveTick`
  (params (DeltaSeconds :type "Float (single-precision)"))
  (`SceneComponent.K2_AddWorldOffset` (`self.DefaultSceneRoot`) (`KismetMathLibrary.MakeVector` (* DeltaSeconds (`self.Speed`) -1.0)) false false)
  (if (and (`self.IsHoverEnabled`) (`self.IsHovered`))
    (bind _output_get (set `self.HoverTime` (+ DeltaSeconds (`self.HoverTime`))))
    (if (>= _output_get (`self.MaxHoverTime`))
      (set `self.HoverTime` 0.0)
      (`self.OnWidgetClicked` (`self.SlideIdx`)))))

(event `self.Sphere.OnComponentBeginOverlap`
  (params (OverlappedComponent :type "PrimitiveComponent Object Reference") (OtherActor :type "Actor Object Reference") (OtherComp :type "PrimitiveComponent Object Reference") (OtherBodyIndex :type Integer) (bFromSweep :type Boolean) (SweepResult :type "HitResult Structure (by ref)"))
  (bind _thumbnailwidget (`self.ThumbnailWidget`))
  (if (`self.IsRespawnable`)
    (set `self.IsRespawnable` false)
    (`SceneComponent.K2_AddWorldOffset` (`self.DefaultSceneRoot`) (`KismetMathLibrary.MakeVector` (`self.RespawnDistance`)) false false)
    (elif (`/Game/Blueprints/UI/PanningWidget/W_PanningThumbnail.IsOpen` (`self.ThumbnailWidget`))
      (`/Game/Blueprints/UI/PanningWidget/W_PanningThumbnail.Close` _thumbnailwidget)
      (set `self.IsRespawnable` true)
      (else
        (`/Game/Blueprints/UI/PanningWidget/W_PanningThumbnail.Open` _thumbnailwidget)))))

(event `self.Widget.OnClicked`
  (params (TouchedComponent :type "PrimitiveComponent Object Reference") (ButtonPressed :type "Key Structure" :default "LeapLeftPinch"))
  (if (== ButtonPressed "LeftMouseButton")
    (set `self.HoverTime` 0.0)
    (`self.OnWidgetClicked` (`self.SlideIdx`))))

(event `self.Widget.OnBeginCursorOver`
  (params (TouchedComponent :type "PrimitiveComponent Object Reference"))
  (set `self.IsHovered` true)
  (set `self.HoverTime` 0.0 :!label _label))

(event `self.Widget.OnEndCursorOver`
  (params (TouchedComponent :type "PrimitiveComponent Object Reference"))
  (set `self.IsHovered` false)
  (goto _label))

(fn `UserConstructionScript`)