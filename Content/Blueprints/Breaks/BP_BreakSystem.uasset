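; Selectable break display actor with header/body text that comes forward and is grabbed by the PWN_Rotate pawn for rotation.
; A left click, or timed hover when Leap Motion is enabled, plays a move sequence and records a BreakSelected analytics event.
; Tick smoothly applies and decays accumulated pitch/yaw input on the mesh.
; ReturnToPosition reverses the sequence and eases the mesh back to its initial rotation.
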(event `MoveFinished`
  (set `self.IsMoving` false))

(event `self.ReceiveBeginPlay`
  ;[1 1 1] Init
  (bind _asbp_game_instance (cast `/Game/Blueprints/Game/BP_GameInstance` (`GameplayStatics.GetGameInstance`)))
  (set `self.CanBeHovered` (`.UseLeapMotion_1_9C9D09F642CD68D7D30520AA880A19A8` (break `/Game/Blueprints/Game/S_GameSettings` (`/Game/Blueprints/Game/BP_GameInstance.CurrentGameSettings` _asbp_game_instance))))
  (add `LevelSequencePlayer.OnStop` (`LevelSequenceActor.SequencePlayer` (`self.MoveSequence`)) (delegate `MoveFinished`))
  (bind _aspwn_rotate (cast `/Game/Blueprints/Game/PWN_Rotate` (`Controller.K2_GetPawn` (`GameplayStatics.GetPlayerController` 0))))
  (set `self.ControllingPawn` _aspwn_rotate)
  (set `self.InitialRotation` (`SceneComponent.K2_GetComponentRotation` (`self.StaticMesh`)))
  (bind _asbreak_text (cast `/Game/Blueprints/UI/BreakText` (`WidgetComponent.GetUserWidgetObject` (`self.Text`))))
  (set `/Game/Blueprints/UI/BreakText.HeaderText` (`self.HeaderText`) _asbreak_text)
  (set `/Game/Blueprints/UI/BreakText.BodyText` (`self.BodyText`) _asbreak_text))

(event `self.ReceiveTick`
  (params (DeltaSeconds :type "Float (single-precision)"))
  ;[1 1 1] Tick
  ;;[1 1 1] HoverTimer
  (if (`self.Returning`)
    (`self.ReturnRotate` DeltaSeconds)
    (elif (and (`self.CanBeHovered`) (`self.IsHovered`) (not (`self.IsMoving`)) (`self.CanBeClicked`))
      (bind _output_get (set `self.HoverTime` (+ DeltaSeconds (`self.HoverTime`))))
      (if (>= _output_get (`self.MaxHoverTime`))
        (set `self.HoverTime` 0.0)
        (`self.ComeForward`)
        (`/Game/Blueprints/Game/PWN_Rotate.GrabActor` (`self.ControllingPawn`) self))
      (else
        ;;[1 1 1] Lerp Rotation
        (`self.Rotate(Axis)` (`KismetMathLibrary.FClamp` (* DeltaSeconds (`self.RotateLerpSpeed`))))))))

(event `self.Box.OnBeginCursorOver`
  (params (TouchedComponent :type "PrimitiveComponent Object Reference"))
  ;[1 1 1] Hover
  (set `self.IsHovered` true)
  (set `self.HoverTime` 0.0 :!label _label))

(event `self.Box.OnEndCursorOver`
  (params (TouchedComponent :type "PrimitiveComponent Object Reference"))
  ;[1 1 1] Hover
  (set `self.IsHovered` false)
  (goto _label))

(event `self.Box.OnClicked`
  (params (TouchedComponent :type "PrimitiveComponent Object Reference") (ButtonPressed :type "Key Structure" :default "LeapLeftPinch"))
  ;[1 1 1] Click
  (if (and (== ButtonPressed "LeftMouseButton") (`self.CanBeClicked`) (not (`self.IsMoving`)))
    (`self.ComeForward`)
    (`/Game/Blueprints/Game/PWN_Rotate.GrabActor` (`self.ControllingPawn`) self)))

(fn `AddToTargetRotation`
  (params (RotationVector :type "Rotator Structure"))
  (set `self.TargetRotation` (`KismetMathLibrary.MakeRotator` 0.0 (+ (.pitch RotationVector) (.pitch (`self.TargetRotation`))) (+ (.yaw RotationVector) (.yaw (`self.TargetRotation`))))))

(fn `ComeForward`
  (if (not (`self.IsMoving`))
    (`LevelSequencePlayer.Play` (`LevelSequenceActor.SequencePlayer` (`self.MoveSequence`)))
    (set `self.IsMoving` true)
    (set `self.Returning` false)
    (`AnalyticsBlueprintLibrary.RecordEventWithAttribute` "BreakSelected" "custom2" (`self.HeaderText`))))

(fn `ReturnRotate`
  (params (B :type "Float (double-precision)"))
  (bind _staticmesh (`self.StaticMesh`))
  (bind _returnvalue (`KismetMathLibrary.RLerp` (`SceneComponent.K2_GetComponentRotation` (`self.StaticMesh`)) (`self.InitialRotation`) (* B (`self.ReturnLerpSpeed`)) true))
  (`SceneComponent.K2_SetWorldRotation` _staticmesh _returnvalue false false)
  (if (`KismetMathLibrary.NearlyEqual_FloatFloat` (+ (.roll (`KismetMathLibrary.NormalizedDeltaRotator` (`SceneComponent.K2_GetComponentRotation` _staticmesh) _returnvalue)) (.pitch (`KismetMathLibrary.NormalizedDeltaRotator` (`SceneComponent.K2_GetComponentRotation` _staticmesh) _returnvalue)) (.yaw (`KismetMathLibrary.NormalizedDeltaRotator` (`SceneComponent.K2_GetComponentRotation` _staticmesh) _returnvalue))) 0.0 0.01)
    (set `self.Returning` false)))

(fn `ReturnToPosition`
  (returns (Success :type Boolean))
  (if (not (`self.IsMoving`))
    (`LevelSequencePlayer.PlayReverse` (`LevelSequenceActor.SequencePlayer` (`self.MoveSequence`)))
    (set `self.IsMoving` true)
    (set `self.TargetRotation` (struct))
    (set `self.Returning` true)
    (return true)
    (else
      (return false))))

(fn `Rotate(Axis)`
  (params (Alpha :type "Float (double-precision)"))
  (bind _pitch (.pitch (`self.TargetRotation`)))
  (bind _yaw (.yaw (`self.TargetRotation`)))
  (`SceneComponent.K2_AddWorldRotation` (`self.StaticMesh`) (`KismetMathLibrary.RLerp` (`KismetMathLibrary.ComposeRotators` (`KismetMathLibrary.RotatorFromAxisAndAngle` (0.0 1.0 0.0) _pitch) (`KismetMathLibrary.RotatorFromAxisAndAngle` (0.0 0.0 1.0) _yaw)) (struct) Alpha) false false)
  (set `self.TargetRotation` (`KismetMathLibrary.MakeRotator` 0.0 (`KismetMathLibrary.Lerp` _pitch 0.0 Alpha) (`KismetMathLibrary.Lerp` _yaw 0.0 Alpha))))

(fn `UserConstructionScript`)